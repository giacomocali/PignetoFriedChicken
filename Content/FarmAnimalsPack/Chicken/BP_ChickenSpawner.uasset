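; Chicken spawner actor that releases escalating waves of chickens around itself on a timer.
; Each wave spawns one bird per second up to MaxPolli, mostly BP_Chicken with an occasional BP_ChickenSheriff, at random yaw and horizontal offsets scaled by the Sphere radius.
; After each wave, MaxPolli increases and the looping Spawn timer restarts with a longer interval.
; The construction script's child-actor scattering is disconnected and never runs.
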(event Custom|Spawn
  (bind _transform (CallFunction|GetRandomSpawnTransform))
  (bind _maxpolli (Variables|Default|GetMaxPolli))
  (if (< (Variables|Default|GetIndex) _maxpolli) :!label _label
    (if (<= (Math|Random|RandomInteger 9) 7)
      (Game|SpawnActorfromClass "/Game/FarmAnimalsPack/Chicken/BP_Chicken.BP_Chicken_C" _transform "AdjustIfPossibleButDontSpawnIfColliding" "MultiplyWithRoot" 0 0)
      (else
        (Game|SpawnActorfromClass "/Game/FarmAnimalsPack/Chicken/BP_ChickenSheriff.BP_ChickenSheriff_C" _transform "AdjustIfPossibleButDontSpawnIfColliding" "MultiplyWithRoot" 0 0)))
    (Math|Integer|IncrementInt (Variables|Default|GetIndex)
      (:%20%20
        (Utilities|FlowControl|Delay 1.0)
        (goto _label)))
    (else
      (bind _result (Math|Integer|IncrementInt _maxpolli)
        (:%20%20
          (Variables|Default|SetIndex 0)
          (CallFunction|CustomEvent (+ (* _result 0.25) 5.0)))))))

(event Custom|CustomEvent
  (params (Time :type Float%20%28single-precision%29))
  (Utilities|Time|SetTimerbyFunctionName 0 "Spawn" Time true))

(event EventBeginPlay
  (Utilities|Time|SetTimerbyFunctionName 0 "Spawn" (Variables|Default|GetTime) true))

(fn ConstructionScript)

(fn GetRandomSpawnTransform
  (bind _returnvalue (Math|Random|RandomUnitVector))
  (bind _self self)
  (bind _sphere (Variables|Default|GetSphere))
  (bind _returnvalue_2 (Transformation|GetActorTransform _self))
  (bind _sphereradius (Variables|/Script/Engine.SphereComponent|GetSphereRadius _sphere))
  (bind _returnvalue_3 (* _returnvalue _sphereradius))
  (return (Math|Transform|MakeTransform (+ (Math|Vector|MakeVector (.x _returnvalue_3) (.y _returnvalue_3) 0.0) (.location _returnvalue_2)) (Math|Rotator|MakeRotator 0.0 0.0 (Math|Random|RandomFloatinRange 0.0 3.6e+02)) (/ (.scale _returnvalue_2) "1.000000,1.000000,1.000000"))))