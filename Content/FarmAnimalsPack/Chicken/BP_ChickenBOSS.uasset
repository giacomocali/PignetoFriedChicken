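; Boss chicken enemy character that switches between calm and angry movement, attacks the player and can be killed.
; It drives the Chicken_AnimBP state and speed, seeds its AI controller's blackboard with a random Stream value, and changes walk speed on interface events.
; Tick triggers a timed, DoOnce-gated melee hit when the player is near.
; Incoming damage is scaled down, and death notifies the controller before delayed destruction.
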(event Custom|BPI_Angry_1
  (Variables|/Script/Engine.CharacterMovementComponent|SetMaxWalkSpeed (Variables|Character|GetCharacterMovement) 225.0)
  (Variables|/Game/FarmAnimalsPack/Chicken/Chicken_AnimBP.Chicken_AnimBP_C|SetE_ChckenStates (Variables|Default|GetAs%20Chicken%20Anim%20BP) "NewEnumerator1")
  (Development|PrintString "Hello" false false))

(event Custom|ResetDamage%20DO
  (Utilities|FlowControl|DoOnce false) ; enters at Reset
)

(event Custom|DamagePlayer
  (Variables|/Game/FarmAnimalsPack/Chicken/Chicken_AnimBP.Chicken_AnimBP_C|SetE_ChckenStates (Variables|Default|GetAs%20Chicken%20Anim%20BP) "NewEnumerator2")
  (Utilities|FlowControl|Sequence
    (:then_0
      (Utilities|FlowControl|Delay 0.5)
      (Development|PrintString "POLLO ATTACK")
      (Game|Damage|ApplyDamage (Game|Player|GetPlayerPawn 0) 3.0 0 0))
    (:then_1
      (Utilities|FlowControl|Delay 0.84)
      (Variables|/Game/FarmAnimalsPack/Chicken/Chicken_AnimBP.Chicken_AnimBP_C|SetE_ChckenStates (Variables|Default|GetAs%20Chicken%20Anim%20BP) "NewEnumerator1")
      (Utilities|FlowControl|Delay 1.0)
      (CallFunction|ResetDamageDO))))

(event EventBeginPlay
  (bind _aschicken_anim_bp (Utilities|Casting|CastToChicken_AnimBP (Components|SkeletalMesh|GetAnimInstance (Variables|Character|GetMesh))))
  (Variables|Default|SetAs%20Chicken%20Anim%20BP _aschicken_anim_bp)
  (bind _asai_chicken_controller (Utilities|Casting|CastToAI_ChickenController (Pawn|GetController)))
  (bind _output_get (Variables|Default|SetAs%20AI%20Chicken%20Controller _asai_chicken_controller))
  (Utilities|IsValid (AI|GetBlackboard 0)
    (:Is%20Valid
      _)
    (:Is%20Not%20Valid
      (Utilities|FlowControl|DelayUntilNextTick)))
  (Class|BlackboardComponent|SetValueasInt (Variables|/Script/AIModule.AIController|GetBlackboard _output_get) (Utilities|Name|MakeLiteralName "Stream") (Math|Random|RandomInteger 1000)))

(event EventTick
  (params (DeltaSeconds :type Float%20%28single-precision%29))
  (bind _returnvalue (Game|Player|GetPlayerPawn 0))
  (Variables|/Game/FarmAnimalsPack/Chicken/Chicken_AnimBP.Chicken_AnimBP_C|SetSpeed (Variables|Default|GetAs%20Chicken%20Anim%20BP) (Math|Vector|VectorLength (Transformation|GetVelocity)))
  (Utilities|IsValid _returnvalue
    (:Is%20Valid
      (if (and (<= (Math|Vector|Distance(Vector) (Transformation|GetActorLocation _returnvalue) (Transformation|GetActorLocation)) 4e+02) (Utilities|Enum|NotEqual(Enum) (Variables|/Game/FarmAnimalsPack/Chicken/Chicken_AnimBP.Chicken_AnimBP_C|GetE_ChckenStates (Variables|Default|GetAs%20Chicken%20Anim%20BP)) "NewEnumerator3"))
        (Utilities|FlowControl|DoOnce false :!label _label
          (:Completed
            (CallFunction|DamagePlayer)))
        (else
          (goto _label Reset))))))

(event EventBPICalm
  (Variables|/Script/Engine.CharacterMovementComponent|SetMaxWalkSpeed (Variables|Character|GetCharacterMovement) 125.0)
  (Variables|/Game/FarmAnimalsPack/Chicken/Chicken_AnimBP.Chicken_AnimBP_C|SetE_ChckenStates (Variables|Default|GetAs%20Chicken%20Anim%20BP) "NewEnumerator0")
  (Development|PrintString "Mello" false false))

(event Game|Damage|EventAnyDamage
  (params (Damage :type Float%20%28single-precision%29) (DamageType :type Damage%20Type%20Object%20Reference) (InstigatedBy :type Controller%20Object%20Reference) (DamageCauser :type Actor%20Object%20Reference))
  (bind _output_get (Variables|Default|SetHP (- (Variables|Default|GetHP) (/ Damage 1e+01))))
  (if (<= _output_get 0.0)
    (Variables|/Game/FarmAnimalsPack/Chicken/Chicken_AnimBP.Chicken_AnimBP_C|SetE_ChckenStates (Variables|Default|GetAs%20Chicken%20Anim%20BP) "NewEnumerator3")
    (Default|DeadPawn (Variables|Default|GetAs%20AI%20Chicken%20Controller))
    (Utilities|FlowControl|Delay 1.26)
    (Actor|DestroyActor)))

(fn ConstructionScript)